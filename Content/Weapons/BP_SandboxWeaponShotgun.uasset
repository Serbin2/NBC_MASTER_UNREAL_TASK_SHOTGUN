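; BP_SandboxWeaponShotgun is a shotgun weapon that fires a spread of hitscan pellets.
; SandboxFire checks CanFire and ammo, then plays a sound, runs several line traces at random directions within a cone around FirePoint, and updates ammo.
; It then sets a HandleFireDelay timer from the rate of fire, or reloads with a sound when the ammo check fails.
; BeginPlay also calls Fire after a short delay.
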(event `self.ReceiveBeginPlay`
  (`KismetSystemLibrary.Delay` 0.2)
  (`self.Fire`))

(event `self.SandboxFire`
  (if (`self.CanFire`)
    (bind _returnvalue (`self.CheckAmmo`))
    (if _returnvalue
      (`|ExecutionSequence`
        (:`then_0`
          (`self.PlaySound` null)
          (for _ (range 6)
            (`self.LineTraceOneShot` (`KismetMathLibrary.RandomUnitVectorInConeInDegrees` (`SceneComponent.GetForwardVector` (`self.FirePoint`)) 20.0)))
          (`self.UpdateAmmo`))
        (:`then_1`
          (bind _returnvalue_2 (`KismetSystemLibrary.K2_SetTimer` null "HandleFireDelay" (/ 1.0 (`self.RoF`))))
          (set `self.TimerFireDelay` _returnvalue_2)))
      (else
        (`self.Reload`)
        (`self.PlaySound` null)))))

(fn `UserConstructionScript`)